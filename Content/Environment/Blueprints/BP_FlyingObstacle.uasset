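; BP_FlyingObstacle is an environment obstacle that spins and flies toward a point offset 2000 units in -Y from the player.
; Shortly after BeginPlay it captures that target once and randomizes yaw spin and move duration, so "FlyingSpeed" is really travel time.
; Tick applies the spin and calls latent MoveComponentTo on the root, destroying the actor once its Y drops within 500 units of the target.
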(event EventBeginPlay
  ;[0.49 1 0.4779] Begin play - Get location to move for Obstacle and randomize it's speed and rotation
  (Utilities|FlowControl|Delay 0.2)
  (Variables|Default|SetMoveToLocation (- (Transformation|GetActorLocation (Game|Player|GetPlayerPawn 0)) "0.000000,2000.000000,0.000000"))
  (Variables|Default|SetRotationSpeed (Math|Random|RandomFloatinRange -2.0 2.0))
  (Variables|Default|SetFlyingSpeed (Math|Random|RandomFloatinRange 3.0 12.0)))

(event EventTick
  (params (DeltaSeconds :type Float%20%28single-precision%29))
  ;[1 1 1] Event tick - Move obstacle
  (Transformation|AddLocalRotation (Variables|Default|GetDefaultSceneRoot) (Math|Rotator|MakeRotator 0.0 0.0 (Variables|Default|GetRotationSpeed)) false false)
  (if (< (.y (Transformation|GetActorLocation)) (+ 5e+02 (.y (Variables|Default|GetMoveToLocation))))
    (Actor|DestroyActor)
    (else
      (Components|MoveComponentTo (Variables|Default|GetDefaultSceneRoot) (Variables|Default|GetMoveToLocation) "0, 0, 0" false false (Variables|Default|GetFlyingSpeed) false))))

(fn ConstructionScript)