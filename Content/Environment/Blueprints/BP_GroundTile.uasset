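; BP_GroundTile is a ground tile that extends the level as the player advances.
; When BP_Character overlaps EndTrigger, it asks BP_TopDownGameMode to add the next tile at SpawnPoint's transform.
; Spawn functions, not called here, place enemies and randomly scaled flying obstacles at random points in a box area.
; A third spawns smaller, collision-free rocks at negative heights within a separate area's horizontal bounds.
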(event OnComponentBeginOverlap(EndTrigger)
  (params (OverlappedComponent :type Primitive%20Component%20Object%20Reference) (OtherActor :type Actor%20Object%20Reference) (OtherComp :type Primitive%20Component%20Object%20Reference) (OtherBodyIndex :type Integer) (bFromSweep :type Boolean) (SweepResult :type Hit%20Result%20Structure%20%28by%20ref%29))
  ;[1 1 1] Spawn next Tile after player collision with EndTrigger
  (Utilities|Casting|CastToBP_Character OtherActor)
  (bind _asbp_top_down_game_mode (Utilities|Casting|CastToBP_TopDownGameMode (Game|GetGameMode)))
  (Default|AddGroundTile _asbp_top_down_game_mode (Transformation|GetWorldTransform (Variables|Default|GetSpawnPoint))))

(fn ConstructionScript)

(fn SpawnEnemies
  (bind _enemyandobstaclespawnarea (Variables|Default|GetEnemyAndObstacleSpawnArea))
  (Game|SpawnActorfromClass "/Game/Enemy/Blueprints/BP_Enemy.BP_Enemy_C" (Math|Conversions|ToTransform(Vector) (Math|Random|RandomPointinBoundingBox (Transformation|GetWorldLocation _enemyandobstaclespawnarea) (Variables|/Script/Engine.BoxComponent|GetBoxExtent _enemyandobstaclespawnarea))) "Undefined" "MultiplyWithRoot" 0 0))

(fn SpawnObstacles
  (bind _returnvalue (Math|Random|RandomFloatinRange 0.5 2.0))
  (bind _enemyandobstaclespawnarea (Variables|Default|GetEnemyAndObstacleSpawnArea))
  (bind _returnvalue_2 (Game|SpawnActorfromClass "/Game/Environment/Blueprints/BP_FlyingObstacle.BP_FlyingObstacle_C" (Math|Conversions|ToTransform(Vector) (Math|Random|RandomPointinBoundingBox (Transformation|GetWorldLocation _enemyandobstaclespawnarea) (Variables|/Script/Engine.BoxComponent|GetBoxExtent _enemyandobstaclespawnarea))) "Undefined" "MultiplyWithRoot" 0 0))
  (Transformation|SetActorScale3D _returnvalue_2 (Math|Vector|MakeVector _returnvalue _returnvalue _returnvalue)))

(fn SpawnNonCollisionObstacles
  (bind _returnvalue (Math|Random|RandomFloatinRange 0.05 0.5))
  (bind _noncollisionobstaclesspawnarea (Variables|Default|GetNonCollisionObstaclesSpawnArea))
  (bind _returnvalue_2 (Transformation|GetWorldLocation _noncollisionobstaclesspawnarea))
  (bind _boxextent (Variables|/Script/Engine.BoxComponent|GetBoxExtent _noncollisionobstaclesspawnarea))
  (bind _returnvalue_3 (Math|Random|RandomPointinBoundingBox _returnvalue_2 _boxextent))
  (bind _returnvalue_4 (Game|SpawnActorfromClass "/Game/Environment/Blueprints/BP_FlyingObstacle.BP_FlyingObstacle_C" (Math|Transform|MakeTransform (Math|Vector|MakeVector (.x _returnvalue_3) (.y _returnvalue_3) (Math|Random|RandomFloatinRange -9.5e+02 -5e+02)) "0, 0, 0" "1.000000,1.000000,1.000000") "Undefined" "MultiplyWithRoot" 0 0))
  (Transformation|SetActorScale3D _returnvalue_4 (Math|Vector|MakeVector _returnvalue _returnvalue _returnvalue))
  (Collision|SetCollisionEnabled (Variables|/Game/Environment/Blueprints/BP_FlyingObstacle.BP_FlyingObstacle_C|GetRock _returnvalue_4) "NoCollision"))