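; Player controller for a distance-goal game that runs the HUD, custom cursor and persistent win, loss and kill stats.
; Tick aims BP_Character at the cursor hit, derives distance from focal-point Y, updates the HUD and triggers wins that multiply the target.
; Death records a loss, resets the target and reloads Map01.
; Both outcomes save to SG_PlayerProfile; CheckSaveGame can load it but is never called here.
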(event Custom|PlayerDied
  ;[1 1 1] Player Died
  (Math|Integer|IncrementInt (Variables|SaveGame|GetLosses)
    (:%20%20
      (Variables|Default|SetPlayerProfile (Utilities|Struct|MakeS_PlayerProfile 0 (Variables|SaveGame|GetWins) (Variables|SaveGame|GetLosses) 10000 (Variables|SaveGame|GetTotalKills)))
      (CallFunction|SaveProfile)
      (Widget|SetVisibility (Variables|/Game/Widgets/WB_IngameHUD.WB_IngameHUD_C|GetBorder_PlayerDead (Variables|Default|GetWB_IngameHUD)) "Visible")
      (Utilities|FlowControl|Delay 3.0)
      (Game|OpenLevel(byName) "Map01"))))

(event Custom|UI_UpdateSpeed
  ;[1 1 1] UI Update
  (Rendering|Components|TextRender|SetText (Variables|/Game/Widgets/WB_IngameHUD.WB_IngameHUD_C|GetText_Speed (Variables|Default|GetWB_IngameHUD)) (Utilities|Text|ToText(Float) (Variables|/Game/Character/Blueprints/BP_Character.BP_Character_C|GetCurrentSpeed (Variables|Default|GetBP_Character)) "HalfToEven")))

(event Custom|UI_UpdateKills
  ;[1 1 1] UI Update
  (Math|Integer|IncrementInt (Variables|SaveGame|GetTotalKills)
    (:%20%20
      (Rendering|Components|TextRender|SetText (Variables|/Game/Widgets/WB_IngameHUD.WB_IngameHUD_C|GetText_Kills (Variables|Default|GetWB_IngameHUD)) (Utilities|Text|ToText(Integer) (Variables|SaveGame|GetTotalKills))))))

(event Custom|UI_ShowOutOfBoundsMessage
  ;[1 1 1] UI Out of Bounds
  (Widget|SetVisibility (Variables|/Game/Widgets/WB_IngameHUD.WB_IngameHUD_C|GetBorder_OutOfBounds (Variables|Default|GetWB_IngameHUD)) "Visible")
  (Utilities|FlowControl|Delay 2.0)
  (Widget|SetVisibility (Variables|/Game/Widgets/WB_IngameHUD.WB_IngameHUD_C|GetBorder_OutOfBounds (Variables|Default|GetWB_IngameHUD)) "Hidden"))

(event EventBeginPlay
  ;[0.3787 1 0.428] Begin Play
  (Viewport|RemoveAllWidgets)
  (Variables|Default|SetbShowMouseCursor true)
  (CallFunction|ShowUIHUD)
  (Rendering|Components|TextRender|SetText (Variables|/Game/Widgets/WB_IngameHUD.WB_IngameHUD_C|GetText_Destination (Variables|Default|GetWB_IngameHUD)) (Utilities|Text|FormatText "{a} / 10,000 m" (Variables|SaveGame|GetDestination)))
  (Rendering|Components|TextRender|SetText (Variables|/Game/Widgets/WB_IngameHUD.WB_IngameHUD_C|GetText_WinLose (Variables|Default|GetWB_IngameHUD)) (Utilities|Text|FormatText "{a} / {b}" (Variables|SaveGame|GetWins) (Variables|SaveGame|GetLosses)))
  (Rendering|Components|TextRender|SetText (Variables|/Game/Widgets/WB_IngameHUD.WB_IngameHUD_C|GetText_Kills (Variables|Default|GetWB_IngameHUD)) (Utilities|Text|ToText(Integer) (Variables|SaveGame|GetTotalKills)))
  (bind _asbp_character (Utilities|Casting|CastToBP_Character (Game|Player|GetPlayerPawn 0)))
  (Variables|Default|SetBP_Character _asbp_character))

(event EventTick
  (params (DeltaSeconds :type Float%20%28single-precision%29))
  (bind _wb_ingamehud (Variables|Default|GetWB_IngameHUD))
  ;[1 1 1] Event Tick
  (Class|BPICharacter|Lookat(Message) (Variables|Default|GetBP_Character) (.Location (Collision|BreakHitResult (.HitResult (Game|Player|GetHitResultUnderCursorbyChannel "TraceTypeQuery1" true)))))
  (bind _output_get (Variables|SaveGame|SetDestination (/ (Math|Float|Truncate (.y (Class|PlayerController|GetFocalLocation))) (Variables|Default|GetRateOfChangeOfDistance))))
  (Rendering|Components|TextRender|SetText (Variables|/Game/Widgets/WB_IngameHUD.WB_IngameHUD_C|GetText_Destination _wb_ingamehud) (Utilities|Text|FormatText "{a} / {b} m" _output_get (Variables|SaveGame|GetWinTarget)))
  (Rendering|Components|TextRender|SetText (Variables|/Game/Widgets/WB_IngameHUD.WB_IngameHUD_C|GetText_Speed _wb_ingamehud) (Utilities|Text|ToText(Float) (Variables|/Game/Character/Blueprints/BP_Character.BP_Character_C|GetCurrentSpeed (Variables|Default|GetBP_Character)) "HalfToEven"))
  (if (>= (Variables|SaveGame|GetDestination) (Variables|SaveGame|GetWinTarget))
    (CallFunction|PlayerWin)))

(fn ConstructionScript)

(fn ShowUIHUD
  (Utilities|IsValid (Variables|Default|GetWB_IngameHUD)
    (:Is%20Valid
      _)
    (:Is%20Not%20Valid
      (bind _returnvalue (UserInterface|CreateWidget "/Game/Widgets/WB_IngameHUD.WB_IngameHUD_C" self))
      (Variables|Default|SetWB_IngameHUD _returnvalue)))
  (UserInterface|Viewport|AddtoViewport (Variables|Default|GetWB_IngameHUD) 0)
  (Utilities|IsValid (Variables|Default|GetWB_Cursor)
    (:Is%20Valid
      _)
    (:Is%20Not%20Valid
      (bind _returnvalue_2 (UserInterface|CreateWidget "/Game/Widgets/Cursor/WB_Cursor.WB_Cursor_C" self))
      (Variables|Default|SetWB_Cursor _returnvalue_2)))
  (Class|PlayerController|SetMouseCursorWidget "Default" (Variables|Default|GetWB_Cursor))
  (return))

(fn CheckSaveGame
  (bind _returnvalue (SaveGame|DoesSaveGameExist (Variables|Default|GetPlayerProfile_Slot)))
  (if _returnvalue
    (CallFunction|LoadGame)
    (else
      (CallFunction|SaveProfile)))
  (return))

(fn LoadGame
  (bind _returnvalue (SaveGame|LoadGamefromSlot (Variables|Default|GetPlayerProfile_Slot)))
  (bind _assg_player_profile (Utilities|Casting|CastToSG_PlayerProfile _returnvalue))
  (Variables|Default|SetPlayerProfile (Variables|/Game/Frameworks/SaveGame/SG_PlayerProfile.SG_PlayerProfile_C|GetPlayerProfile _assg_player_profile))
  (Variables|SaveGame|SetDestination (.Destination (Utilities|Struct|BreakS_PlayerProfile (Variables|Default|GetPlayerProfile))))
  (Variables|SaveGame|SetWins (.Wins (Utilities|Struct|BreakS_PlayerProfile (Variables|Default|GetPlayerProfile))))
  (Variables|SaveGame|SetLosses (.Loses (Utilities|Struct|BreakS_PlayerProfile (Variables|Default|GetPlayerProfile))))
  (Variables|SaveGame|SetWinTarget (.WinTarget (Utilities|Struct|BreakS_PlayerProfile (Variables|Default|GetPlayerProfile))))
  (Variables|SaveGame|SetTotalKills (.TotalKills (Utilities|Struct|BreakS_PlayerProfile (Variables|Default|GetPlayerProfile))))
  (return))

(fn SaveProfile
  (Utilities|IsValid (Variables|Default|GetSG_PlayerProfile)
    (:Is%20Valid
      _)
    (:Is%20Not%20Valid
      (bind _returnvalue (SaveGame|CreateSaveGameObject "/Game/Frameworks/SaveGame/SG_PlayerProfile.SG_PlayerProfile_C"))
      (Variables|Default|SetSG_PlayerProfile _returnvalue)))
  (Variables|/Game/Frameworks/SaveGame/SG_PlayerProfile.SG_PlayerProfile_C|SetPlayerProfile (Variables|Default|GetSG_PlayerProfile) (Variables|Default|GetPlayerProfile))
  (SaveGame|SaveGametoSlot (Variables|Default|GetSG_PlayerProfile) (Variables|Default|GetPlayerProfile_Slot))
  (return))

(fn PlayerWin
  (Math|Integer|IncrementInt (Variables|SaveGame|GetWins)
    (:%20%20
      (Variables|SaveGame|SetWinTarget (* (Variables|Default|GetDistanceMultiplierForWin) (Variables|SaveGame|GetWinTarget)))
      (Rendering|Components|TextRender|SetText (Variables|/Game/Widgets/WB_IngameHUD.WB_IngameHUD_C|GetText_WinLose (Variables|Default|GetWB_IngameHUD)) (Utilities|Text|FormatText "{a} / {b}" (Variables|SaveGame|GetWins) (Variables|SaveGame|GetLosses)))
      (Variables|Default|SetPlayerProfile (Utilities|Struct|MakeS_PlayerProfile (Variables|SaveGame|GetDestination) (Variables|SaveGame|GetWins) (Variables|SaveGame|GetLosses) (Variables|SaveGame|GetWinTarget) (Variables|SaveGame|GetTotalKills)))
      (CallFunction|SaveProfile))))