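; BP_Enemy is an enemy that chases the player, fires projectiles and reports a kill to the player's UI on death.
; Tick turns it toward the player and drives the chase; within fire range it also orbits at a randomized radius, speed and direction, shooting through a DoOnce gate reset after a delay.
; Sphere overlaps with flying obstacles or the player dash it away.
; Damage updates a widget health bar, and health regenerates after a hit-free delay.
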(event OnComponentBeginOverlap(Sphere)
  (params (OverlappedComponent :type Primitive%20Component%20Object%20Reference) (OtherActor :type Actor%20Object%20Reference) (OtherComp :type Primitive%20Component%20Object%20Reference) (OtherBodyIndex :type Integer) (bFromSweep :type Boolean) (SweepResult :type Hit%20Result%20Structure%20%28by%20ref%29))
  (bind _bp_character (Variables|Default|GetBP_Character))
  ;[1 1 1] Enemy Dash Player and Obstacles
  (bind _asbp_flying_obstacle (Utilities|Casting|CastToBP_FlyingObstacle OtherActor)
    (:then
      (Variables|Movement|SetDashLocation (- (Transformation|GetActorLocation) (* (Class|KismetMathLibrary|VectorNormal2D (- (Transformation|GetActorLocation) (Transformation|GetActorLocation _asbp_flying_obstacle)) 0.1) (Variables|Movement|GetDashDistance) -1)))
      (Components|MoveComponentTo (Variables|Default|GetDefaultSceneRoot) (Variables|Movement|GetDashLocation) (Transformation|GetActorRotation) false false (Variables|Movement|GetDashSpeed) false :!label _label))
    (:CastFailed
      (if (== OtherActor _bp_character)
        (Variables|Movement|SetDashLocation (- (Transformation|GetActorLocation) (* (Class|KismetMathLibrary|VectorNormal2D (- (Transformation|GetActorLocation) (Transformation|GetActorLocation _bp_character)) 0.1) (Variables|Movement|GetDashDistance) -1)))
        (goto _label)))))

(event Custom|UnlockAttack
  (bind _arrow (Variables|Default|GetArrow))
  (bind _arrow_2 (Variables|Default|GetArrow))
  (bind _returnvalue (Transformation|GetWorldLocation _arrow_2))
  ;[1 1 1] Attack
  (Utilities|FlowControl|DoOnce false) ; enters at Reset
)

(event Custom|OnTakeAnyDamage_Event
  (params (DamagedActor :type Actor%20Object%20Reference) (Damage :type Float%20%28single-precision%29) (DamageType :type Damage%20Type%20Object%20Reference) (InstigatedBy :type Controller%20Object%20Reference) (DamageCauser :type Actor%20Object%20Reference))
  ;[1 1 1] On Take Damage
  (Variables|EnemyShip|SetCurrentHealth (- (Variables|EnemyShip|GetCurrentHealth) Damage))
  (Variables|Combat|SetIsTakenDamage true)
  (Variables|Combat|SetElapsedTimeAfterDamage 0.0)
  (CallFunction|UpdateHealthBar)
  (if (<= (Variables|EnemyShip|GetCurrentHealth) 0.0)
    (Default|UIUpdateKills (Variables|/Game/Character/Blueprints/BP_Character.BP_Character_C|GetBP_PlayerController (Variables|Default|GetBP_Character)))
    (Actor|DestroyActor)))

(event EventAttack
  (bind _arrow (Variables|Default|GetArrow))
  (bind _arrow_2 (Variables|Default|GetArrow))
  (bind _returnvalue (Transformation|GetWorldLocation _arrow_2))
  ;[1 1 1] Attack
  (Utilities|FlowControl|DoOnce false
    (:Completed
      (Utilities|FlowControl|Sequence
        (:then_0
          (bind _returnvalue_2 (Game|SpawnActorfromClass "/Game/Enemy/Blueprints/BP_EnemyProjectile.BP_EnemyProjectile_C" (Math|Conversions|ToTransform(Vector) _returnvalue) "Undefined" "MultiplyWithRoot" 0 0))
          (Default|Moveto _returnvalue_2 (+ (Transformation|GetWorldLocation _arrow) (* (Math|Vector|GetForwardVector _arrow) (Variables|Combat|GetProjectileRange))) (Variables|Combat|GetProjectileSpeed))
          (Audio|PlaySoundatLocation "/Game/Enemy/Assets/Sounds/EnemyShot_Cue.EnemyShot_Cue" _returnvalue "0, 0, 0" 0.7 0.1 0.0 0 0 0 0))
        (:then_1
          (Utilities|FlowControl|Delay (Variables|Combat|GetFireRate))
          (CallFunction|UnlockAttack))))))

(event EventTick
  (params (DeltaSeconds :type Float%20%28single-precision%29))
  (bind _returnvalue (Game|Player|GetPlayerPawn 0))
  (bind _returnvalue_2 (Transformation|GetActorLocation _returnvalue))
  ;[1 1 1] Event tick
  (Transformation|SetActorRotation (Class|KismetMathLibrary|RInterptoConstant (Transformation|GetActorRotation) (Variables|Movement|GetTargetRotation) DeltaSeconds 2.7e+02))
  (if (Variables|Combat|GetIsTakenDamage)
    (Variables|Combat|SetElapsedTimeAfterDamage (+ DeltaSeconds (Variables|Combat|GetElapsedTimeAfterDamage)))
    (if (>= (Variables|Combat|GetElapsedTimeAfterDamage) (Variables|EnemyShip|GetSecondsToRegeneration))
      (CallFunction|RegenerateHealth)))
  (Class|BPICharacter|Lookat(Message) self _returnvalue_2)
  (if (>= (Transformation|GetDistanceTo _returnvalue) (Variables|Combat|GetFireRange))
    _
    (else
      (CallFunction|Attack)
      (CallFunction|OrbitingPlayer DeltaSeconds)))
  (Components|MoveComponentTo (Variables|Default|GetDefaultSceneRoot) _returnvalue_2 (Transformation|GetActorRotation) true false (Variables|Movement|GetChaseSpeed) false))

(event EventLookat
  (params (Target :type Vector :default "0, 0, 0"))
  (bind _returnvalue (Transformation|GetActorLocation))
  ;[1 1 1] Look At
  (Variables|Movement|SetTargetRotation (Math|Rotator|FindLookatRotation (Math|Vector|MakeVector (.x Target) (.y Target) 0.0) (Math|Vector|MakeVector (.x _returnvalue) (.y _returnvalue) 0.0))))

(event EventBeginPlay
  ;[0.3875 1 0.5055] Begin Play
  (EventDispatchers|AssignOnTakeAnyDamage (EventDispatchers|CreateEvent :!event Custom|OnTakeAnyDamage_Event))
  (CallFunction|UpdateHealthBar)
  (Variables|Movement|SetRotationSpeed (* (Math|Random|RandomFloatinRange 2e+01 8e+01) (Math|Integer|SelectInt 1 -1 (Math|Random|RandomBool))))
  (Variables|Movement|SetOrbitingPlayerRadius (Math|Random|RandomFloatinRange 7e+02 1.5e+03))
  (bind _asbp_character (Utilities|Casting|CastToBP_Character (Game|Player|GetPlayerPawn 0)))
  (Variables|Default|SetBP_Character _asbp_character))

(fn ConstructionScript)

(fn OrbitingPlayer
  (params (DeltaTime :type Float%20%28single-precision%29))
  (bind _returnvalue (Game|Player|GetPlayerPawn 0))
  (bind _returnvalue_2 (Transformation|GetActorLocation _returnvalue))
  (Variables|Movement|SetAngle (+ (* DeltaTime (Variables|Movement|GetRotationSpeed)) (Variables|Movement|GetAngle)))
  (Variables|Movement|SetTargetPositionOrbiting (Math|Vector|MakeVector (+ (* (Variables|Movement|GetOrbitingPlayerRadius) (Math|Trig|Cos(Degrees) (Variables|Movement|GetAngle))) (.x (Transformation|GetActorLocation (Game|Player|GetPlayerPawn 0)))) (+ (* (Variables|Movement|GetOrbitingPlayerRadius) (Math|Trig|Sin(Degrees) (Variables|Movement|GetAngle))) (.y _returnvalue_2)) (.z _returnvalue_2)))
  (Transformation|SetActorLocation (Math|Interpolation|VInterptoConstant (Transformation|GetActorLocation) (Variables|Movement|GetTargetPositionOrbiting) DeltaTime 2e+03) false false))

(fn UpdateHealthBar
  (bind _aswb_health_bar (Utilities|Casting|CastToWB_HealthBar (UserInterface|GetUserWidgetObject (Variables|Default|GetHealthBarWidget))))
  (Variables|/Game/Widgets/WB_HealthBar.WB_HealthBar_C|SetHealth _aswb_health_bar (/ (Variables|EnemyShip|GetCurrentHealth) (Variables|EnemyShip|GetMaxHealth))))

(fn RegenerateHealth
  (if (< (Variables|EnemyShip|GetCurrentHealth) (Variables|EnemyShip|GetMaxHealth))
    (Variables|EnemyShip|SetCurrentHealth (+ (Variables|EnemyShip|GetCurrentHealth) (Variables|EnemyShip|GetRegenarationAmount)))
    (CallFunction|UpdateHealthBar)
    (else
      (Variables|Combat|SetIsTakenDamage false))))